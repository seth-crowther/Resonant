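; Player controller for a fighting game that turns Enhanced Input actions into actions on the possessed BP_Fighter.
; Initialize caches the pawn and its state machine, then adds the input mapping context.
; Attack inputs go to the fighter's AttackManager with the current state name.
; Movement, crouch, jump, dodge and parry are gated by the current state, setting horizontal direction or switching states directly.
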(event Custom|Initialize
  ;[1 1 1] Initialize
  (bind _asbp_fighter (Utilities|Casting|CastToBP_Fighter (Pawn|GetControlledPawn)))
  (bind _output_get (Variables|Default|Setfighter _asbp_fighter))
  (Variables|Default|SetstateMachine (Variables|/Script/Resonant.Fighter|GetstateMachine _output_get))
  (CallFunction|InitializeMappingContext))

(event Input|EnhancedActionEvents|EnhancedInputActionIA_DodgeLeft
  (params (ActionValue :type Float%20%28double-precision%29) (ElapsedSeconds :type Float%20%28double-precision%29) (TriggeredSeconds :type Float%20%28double-precision%29) (InputAction :type Input%20Action%20Object%20Reference :default "/Game/Inputs/IA_DodgeLeft.IA_DodgeLeft"))
  ;[1 1 1] Dodging
  (:Started
    (switch Utilities|FlowControl|Switch|SwitchonFighterStateName (Variables|/Script/Resonant.StateMachine|GetcurrentStateName (Variables|Default|GetstateMachine))
      (:Walking
        (Class|StateMachine|SwitchState (Variables|Default|GetstateMachine) "Dodging")))))

(event Input|EnhancedActionEvents|EnhancedInputActionIA_Square
  (params (ActionValue :type Boolean) (ElapsedSeconds :type Float%20%28double-precision%29) (TriggeredSeconds :type Float%20%28double-precision%29) (InputAction :type Input%20Action%20Object%20Reference :default "/Game/Inputs/IA_Square.IA_Square"))
  (bind _statemachine (Variables|Default|GetstateMachine))
  ;[1 1 1] Parry
  (:Started
    (switch Utilities|FlowControl|Switch|SwitchonFighterStateName (Variables|/Script/Resonant.StateMachine|GetcurrentStateName _statemachine)
      (:Walking
        (Class|StateMachine|SwitchState _statemachine "Parrying")))))

(event Input|EnhancedActionEvents|EnhancedInputActionIA_R1
  (params (ActionValue :type Boolean) (ElapsedSeconds :type Float%20%28double-precision%29) (TriggeredSeconds :type Float%20%28double-precision%29) (InputAction :type Input%20Action%20Object%20Reference :default "/Game/Inputs/IA_R1.IA_R1"))
  ;[1 1 1] Sweep attack
  (:Started
    (Default|AttackInput (Variables|/Game/Blueprints/BP_Fighter.BP_Fighter_C|GetAttackManager (Variables|Default|Getfighter)) InputAction (Variables|/Script/Resonant.StateMachine|GetcurrentStateName (Variables|Default|GetstateMachine)))))

(event Input|EnhancedActionEvents|EnhancedInputActionIA_LeftStickHorizontal
  (params (ActionValue :type Float%20%28double-precision%29) (ElapsedSeconds :type Float%20%28double-precision%29) (TriggeredSeconds :type Float%20%28double-precision%29) (InputAction :type Input%20Action%20Object%20Reference :default "/Game/Inputs/IA_LeftStickHorizontal.IA_LeftStickHorizontal"))
  ;[1 1 1] Left stick input
  (:Triggered
    (if (Utilities|Enum|Equal(Enum) (Variables|/Script/Resonant.StateMachine|GetcurrentStateName (Variables|Default|GetstateMachine)) "Walking")
      (Variables|/Game/Blueprints/BP_Fighter.BP_Fighter_C|SethorizontalMoveDir (Variables|Default|Getfighter) (Math|Float|Round ActionValue))))
  (:Canceled
    (Variables|/Game/Blueprints/BP_Fighter.BP_Fighter_C|SethorizontalMoveDir (Variables|Default|Getfighter) 0 :!label _label))
  (:Completed
    (goto _label)))

(event Input|EnhancedActionEvents|EnhancedInputActionIA_LeftStickVertical
  (params (ActionValue :type Float%20%28double-precision%29) (ElapsedSeconds :type Float%20%28double-precision%29) (TriggeredSeconds :type Float%20%28double-precision%29) (InputAction :type Input%20Action%20Object%20Reference :default "/Game/Inputs/IA_LeftStickVertical.IA_LeftStickVertical"))
  (bind _returnvalue (Math|Float|Round ActionValue))
  (bind _returnvalue_2 (== _returnvalue -1))
  ;[1 1 1] Crouching
  (:Triggered
    (switch Utilities|FlowControl|Switch|SwitchonFighterStateName (Variables|/Script/Resonant.StateMachine|GetcurrentStateName (Variables|Default|GetstateMachine))
      (:Walking
        (if _returnvalue_2
          (Class|StateMachine|SwitchState (Variables|Default|GetstateMachine) "Crouching")))
      (:Crouching
        (if (not _returnvalue_2)
          (Class|StateMachine|SwitchState (Variables|Default|GetstateMachine) "Walking")))))
  (:Canceled
    (if (Utilities|Enum|Equal(Enum) (Variables|/Script/Resonant.StateMachine|GetcurrentStateName (Variables|Default|GetstateMachine)) "Crouching") :!label _label
      (Class|StateMachine|SwitchState (Variables|Default|GetstateMachine) "Walking")))
  (:Completed
    (goto _label)))

(event Input|EnhancedActionEvents|EnhancedInputActionIA_Cross
  (params (ActionValue :type Boolean) (ElapsedSeconds :type Float%20%28double-precision%29) (TriggeredSeconds :type Float%20%28double-precision%29) (InputAction :type Input%20Action%20Object%20Reference :default "/Game/Inputs/IA_Cross.IA_Cross"))
  ;[1 1 1] Jumping
  (:Started
    (switch Utilities|FlowControl|Switch|SwitchonFighterStateName (Variables|/Script/Resonant.StateMachine|GetcurrentStateName (Variables|Default|GetstateMachine))
      (:Walking
        _)
      (:Crouching
        _))
    (Class|StateMachine|SwitchState (Variables|Default|GetstateMachine) "Jumping")))

(event Input|EnhancedActionEvents|EnhancedInputActionIA_L1
  (params (ActionValue :type Boolean) (ElapsedSeconds :type Float%20%28double-precision%29) (TriggeredSeconds :type Float%20%28double-precision%29) (InputAction :type Input%20Action%20Object%20Reference :default "/Game/Inputs/IA_L1.IA_L1"))
  ;[1 1 1] Left punch attack
  (:Started
    (Default|AttackInput (Variables|/Game/Blueprints/BP_Fighter.BP_Fighter_C|GetAttackManager (Variables|Default|Getfighter)) InputAction (Variables|/Script/Resonant.StateMachine|GetcurrentStateName (Variables|Default|GetstateMachine)))))

(event Input|EnhancedActionEvents|EnhancedInputActionIA_R2
  (params (ActionValue :type Boolean) (ElapsedSeconds :type Float%20%28double-precision%29) (TriggeredSeconds :type Float%20%28double-precision%29) (InputAction :type Input%20Action%20Object%20Reference :default "/Game/Inputs/IA_R2.IA_R2"))
  ;[1 1 1] Right Knee Attack
  (:Started
    (Default|AttackInput (Variables|/Game/Blueprints/BP_Fighter.BP_Fighter_C|GetAttackManager (Variables|Default|Getfighter)) InputAction (Variables|/Script/Resonant.StateMachine|GetcurrentStateName (Variables|Default|GetstateMachine)))))

(fn ConstructionScript)

(fn InitializeMappingContext
  (bind _self self)
  (bind _returnvalue (PlayerController|LocalPlayerSubsystems|GetEnhancedInputLocalPlayerSubsystem _self))
  (Utilities|IsValid _returnvalue
    (:Is%20Valid
      (Input|AddMappingContext _returnvalue "/Game/Inputs/PlayerInputMappingContext.PlayerInputMappingContext" 0 "(bIgnoreAllPressedKeysUntilRelease=True,bForceImmediately=False)"))))