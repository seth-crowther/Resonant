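; Player pawn with hand-written side-on movement: walking along the Y axis and jumping along Z, driven by Enhanced Input.
; Move input sets a horizontal direction, and a jump locks that direction for the whole airtime.
; Tick applies swept location changes, integrating gravity only while airborne.
; Only a downward hit on a perfectly flat surface restores the grounded state; nothing clears it except jumping.
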(event Input|EnhancedActionEvents|EnhancedInputActionIA_Move
  (params (ActionValue :type Float%20%28double-precision%29) (ElapsedSeconds :type Float%20%28double-precision%29) (TriggeredSeconds :type Float%20%28double-precision%29) (InputAction :type Input%20Action%20Object%20Reference :default "/Game/Inputs/IA_Move.IA_Move"))
  ;[1 1 1] Getting Left Stick Input
  (:Triggered
    (if (> ActionValue 0.0)
      (Variables|Default|SethorizontalInputDir 1)
      (else
        (Variables|Default|SethorizontalInputDir -1))))
  (:Completed
    (Variables|Default|SethorizontalInputDir 0)))

(event Input|EnhancedActionEvents|EnhancedInputActionIA_Jump
  (params (ActionValue :type Boolean) (ElapsedSeconds :type Float%20%28double-precision%29) (TriggeredSeconds :type Float%20%28double-precision%29) (InputAction :type Input%20Action%20Object%20Reference :default "/Game/Inputs/IA_Jump.IA_Jump"))
  ;[1 1 1] Handle Jumping
  (:Started
    (if (Variables|Default|GetisGrounded)
      (Variables|Default|SetzSpeed 4e+02)
      (Variables|Default|SetisGrounded false)
      (Variables|Default|SetlastHorizontalDir (Variables|Default|GethorizontalInputDir)))))

(event EventBeginPlay
  ;[1 1 1] Initialising Input Mapping Context
  (bind _asplayer_controller (Utilities|Casting|CastToPlayerController (Pawn|GetController)))
  (Utilities|IsValid (PlayerController|LocalPlayerSubsystems|GetEnhancedInputLocalPlayerSubsystem _asplayer_controller)
    (:Is%20Valid
      (Input|AddMappingContext (PlayerController|LocalPlayerSubsystems|GetEnhancedInputLocalPlayerSubsystem _asplayer_controller) "/Game/Inputs/PlayerInputMappingContext.PlayerInputMappingContext" 0 "(bIgnoreAllPressedKeysUntilRelease=True,bForceImmediately=False)"))))

(event EventTick
  (params (DeltaSeconds :type Float%20%28single-precision%29))
  (bind _returnvalue (Transformation|GetActorLocation))
  (bind _returnvalue_2 (Transformation|GetActorLocation))
  (bind (_x _y _z) (Math|Vector|BreakVector _returnvalue_2))
  (bind (_x_2 _y_2 _z_2) (Math|Vector|BreakVector _returnvalue))
  (if (Variables|Default|GetisGrounded)
    ;[1 1 1] Handle Grounded Movement
    (Transformation|SetActorLocation (Math|Vector|MakeVector _x (+ (* DeltaSeconds (Variables|Default|GetwalkingSpeed) (Variables|Default|GethorizontalInputDir)) _y) _z) true false)
    (else
      ;[1 1 1] Handle Airborne Movement
      (Variables|Default|SetzSpeed (+ (* (Variables|Default|Getgravity) DeltaSeconds) (Variables|Default|GetzSpeed)))
      (Transformation|SetActorLocation (Math|Vector|MakeVector _x_2 (+ _y_2 (* DeltaSeconds (Variables|Default|GetwalkingSpeed) (Variables|Default|GetlastHorizontalDir))) (+ _z_2 (* (Variables|Default|GetzSpeed) DeltaSeconds))) true false))))

(event Collision|EventHit
  (params (MyComp :type Primitive%20Component%20Object%20Reference) (Other :type Actor%20Object%20Reference) (OtherComp :type Primitive%20Component%20Object%20Reference) (bSelfMoved :type Boolean) (HitLocation :type Vector :default "0, 0, 0") (HitNormal :type Vector :default "0, 0, 0") (NormalImpulse :type Vector :default "0, 0, 0") (Hit :type Hit%20Result%20Structure%20%28by%20ref%29))
  ;[1 1 1] Reset Z Speed When Hitting Ground
  (if (and (< (Variables|Default|GetzSpeed) 0.0) (== (.Z (Class|KismetMathLibrary|BreakVector3f HitNormal)) 1.0))
    (Variables|Default|SetzSpeed 0.0)
    (Variables|Default|SetisGrounded true)))

(fn ConstructionScript)