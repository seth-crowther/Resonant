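; Attack component for a fighter in a rhythm-based fighting game, rewarding attacks input on the Speaker's beat.
; Input selects an attack from standing, crouched or aerial sets and plays its montage at a Speaker-derived rate.
; HitDetect sphere-traces at the attack's bone, resolving attack height against the opponent's state.
; Confirmed hits deal damage and beat-based stun; on-beat hits raise damage amplification, which off-beat or premature inputs reset.
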(event Custom|AttackInput
  (params (InputAction :type Input%20Action%20Object%20Reference) (currentState :type FighterStateName%20Enum :default "Walking"))
  (Utilities|ExecuteAttack InputAction currentState))

(event EventBeginPlay
  (bind _asgmb_fight (Utilities|Casting|CastToGMB_Fight (Game|GetGameMode)))
  (Variables|Default|Setspeaker (Variables|/Game/Setup/GMB_Fight.GMB_Fight_C|Getspeaker _asgmb_fight)))

(fn HitDetect
  (bind _owner (Variables|Default|Getowner))
  (bind _opponent (Variables|Default|Getopponent))
  (bind _activeattack (Variables|Default|GetactiveAttack))
  (bind _activeattack_2 (Variables|Default|GetactiveAttack))
  (bind (_animation _damage _targetbone _immobilizehorizontal _immobilizevertical _height) (Utilities|Struct|BreakAttack _activeattack_2))
  (bind (_animation_2 _damage_2 _targetbone_2 _immobilizehorizontal_2 _immobilizevertical_2 _height_2 _inputaction _beatstostun) (Utilities|Struct|BreakAttack _activeattack))
  (bind _mesh (Variables|/Game/Blueprints/BP_Fighter.BP_Fighter_C|GetMesh _owner))
  (bind _returnvalue (Transformation|GetSocketLocation _mesh _targetbone))
  (if (not (Variables|Flags|GethasHitAlready))
    (bind _outhit (Collision|SphereTraceForObjects _returnvalue _returnvalue 1e+01 (Utilities|Array|MakeArray "ObjectTypeQuery3") false 0 "ForDuration"))
    (Utilities|IsValid (.HitComponent (Collision|BreakHitResult _outhit))
      (:Is%20Valid
        (if (== (Components|GetOwner (.HitComponent (Collision|BreakHitResult _outhit))) _opponent)
          (bind _hit (CallFunction|HitConnected _opponent _height))
          (if _hit
            (Variables|Flags|SethasHitAlready true) ; At this point, the hit is confirmed
            (if (Variables|Flags|GetinputOnBeat)
              (Default|IncreaseDamageAmp (Variables|Default|Getowner) 0.1))
            (Default|GetHit (Variables|Default|Getopponent) _damage_2 _beatstostun _height_2)))))))

(fn ResetAmp
  (Variables|/Game/Blueprints/BP_Fighter.BP_Fighter_C|SetdamageAmplifier (Variables|Default|Getowner) 0.0)
  (Variables|Flags|SetinputOnBeat false))

(fn CheckInputBeat
  (if (and (Variables|Flags|GetcanAttackAgain) (Variables|/Script/Resonant.MusicManager|GetonBeat (Variables|Default|Getspeaker)))
    (Variables|Flags|SetinputOnBeat true)
    (else
      (CallFunction|ResetAmp))))

(fn SetActiveAttack
  (params (attackArray :type Array%20of%20Attack%20Structures) (inputAction :type Input%20Action%20Object%20Reference))
  (for _array_element attackArray
    (if (== (.inputAction (Utilities|Struct|BreakAttack _array_element)) inputAction)
      (Variables|Default|SetactiveAttack _array_element)
      (Variables|Flags|SetisActiveAttackValid true)
      (return)))
  (Variables|Flags|SetisActiveAttackValid false))

(fn HitConnected
  (params (Enemy :type BP%20Fighter%20Object%20Reference) (AttackHeight :type AttackHeight%20Enum :default "None"))
  (bind _statemachine (Variables|/Script/Resonant.Fighter|GetstateMachine Enemy))
  (bind _currentstatename (Variables|/Script/Resonant.StateMachine|GetcurrentStateName _statemachine))
  (switch Utilities|FlowControl|Switch|SwitchonAttackHeight AttackHeight
    (:None
      _)
    (:Low
      (switch Utilities|FlowControl|Switch|SwitchonFighterStateName _currentstatename
        (:Walking
          (return true))
        (:Crouching
          _)
        (:Jumping
          _)
        (:Parrying
          (return true))
        (:Dodging
          _)
        (:Hitstun
          (return true))))
    (:High
      (switch Utilities|FlowControl|Switch|SwitchonFighterStateName _currentstatename
        (:Walking
          (return true))
        (:Crouching
          _)
        (:Jumping
          _)
        (:Parrying
          _)
        (:Dodging
          _)
        (:Hitstun
          (return true))))
    (:Aerial
      (switch Utilities|FlowControl|Switch|SwitchonFighterStateName _currentstatename
        (:Walking
          (return true))
        (:Crouching
          (return true))
        (:Jumping
          (return true))
        (:Parrying
          _)
        (:Dodging
          _)
        (:Hitstun
          (return true)))))
  (return false))