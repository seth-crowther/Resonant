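; Fighting-game camera actor that keeps both fighters in frame and becomes the player's view target on BeginPlay.
; It gets the left and right characters from the level's Brain_BP.
; Each tick it moves back along its forward vector from their Y/Z midpoint, raised by a height tweak.
; Pullback distance uses half their Y separation, a padding tweak and the tangent of half the FOV, clamped to a minimum.
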(event EventBeginPlay
  (CallFunction|GetBrainBP)
  (Game|Player|SetViewTargetwithBlend (Game|GetPlayerController 0) self 0.0 "VTBlend_Linear" 0.0 false))

(event EventTick
  (params (DeltaSeconds :type Float%20%28single-precision%29))
  (Transformation|SetActorLocation (+ (Utilities|GetCharMidpoint) (Utilities|MultiplyVectorFloat (Utilities|MultiplyVectorFloat (Transformation|GetActorForwardVector) -1.0) (Math|Float|Clamp(Float) (Utilities|GetDistBack) (Variables|Default|GetminDistBack) 1e+04))) false false))

(fn ConstructionScript)

(fn GetBrainBP
  (bind _outactors (Actor|GetAllActorsOfClass "/Game/Blueprints/Brain_BP.Brain_BP_C"))
  (Variables|Default|SetbrainBP (Utilities|Array|Get(acopy) _outactors)))