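; Playable fighter Blueprint for a round-based fighting game, handling movement, attacks, hit reactions, parry, dodge and death.
; A state machine selects grounded or airborne movement on Tick, while AttackManager receives montage-based standing attacks with damage, height and stun values.
; Hits trigger stuns timed in music beats from the game mode's BPM, or death, which resets health and advances the round.
; All hit heights currently share one reaction montage, and IncreaseDamageAmp's logic is disconnected.
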(event Custom|GetHitAtHeight
  (params (Hit%20Type :type PossibleHits%20Enum :default "NewEnumerator0"))
  (Utilities|ExecuteHitReaction Hit%20Type))

(event EventBeginPlay
  (CallFunction|InitialiseAttacks)
  (Class|SkeletalMeshComponent|SetAnimClass (Variables|Default|GetMesh) "/Game/Animations/Control/Character_AnimationBlueprint.Character_AnimationBlueprint_C"))

(event EventDodge
  (Utilities|HandleDodge))

(event EventStartGameplay
  ;[1 1 1] Only allow input once gameplay has begun - allow input is fired in FightCamera.cpp after intro is complete.
  (bind _aspc_fighter (Utilities|Casting|CastToPC_Fighter (Pawn|GetController)))
  (Default|InitializeMappingContext _aspc_fighter)
  (bind _asgmb_fight (Utilities|Casting|CastToGMB_Fight (Game|GetGameMode)))
  (Variables|/Script/Resonant.FightGameMode|SethasGameplayStarted _asgmb_fight true))

(event EventTick
  (params (DeltaSeconds :type Float%20%28single-precision%29))
  ;[1 1 1] Update
  (if (<= (Variables|Stats|Gethealth) 0.0)
    (Utilities|FlowControl|DoOnce false)
    (else
      (switch Utilities|FlowControl|Switch|SwitchonFighterStateName (Variables|/Script/Resonant.StateMachine|GetcurrentStateName (Variables|Default|GetstateMachine))
        (:Walking
          (Class|Fighter|HandleGroundedMovement DeltaSeconds))
        (:Jumping
          (Class|Fighter|HandleAirborneMovement DeltaSeconds))))))

(event EventStun
  (params (stunBeats :type Float%20%28single-precision%29))
  (Utilities|StunforBeats stunBeats))

(event Collision|EventHit
  (params (MyComp :type Primitive%20Component%20Object%20Reference) (Other :type Actor%20Object%20Reference) (OtherComp :type Primitive%20Component%20Object%20Reference) (bSelfMoved :type Boolean) (HitLocation :type Vector :default "0, 0, 0") (HitNormal :type Vector :default "0, 0, 0") (NormalImpulse :type Vector :default "0, 0, 0") (Hit :type Hit%20Result%20Structure%20%28by%20ref%29))
  ;[1 1 1] Handle Landing
  (if (and (< (Variables|Default|GetzSpeed) 0.0) (== (.Z (Class|KismetMathLibrary|BreakVector3f HitNormal)) 1.0))
    (Class|StateMachine|SwitchState (Variables|Default|GetstateMachine) "Walking")
    (Variables|/Game/Blueprints/AC_AttackManager.AC_AttackManager_C|SetcanAttackAgain (Variables|Default|GetAttackManager) true)))

(event EventParry
  (Utilities|HandleParry))

(event EventSetCanAttack
  (params (value :type Boolean))
  (Variables|/Game/Blueprints/AC_AttackManager.AC_AttackManager_C|SetcanAttackAgain (Variables|Default|GetAttackManager) value))

(event EventPlayIntroAnimation
  (Variables|Default|SethorizontalMoveDir (Variables|Default|Getside))
  (Animation|Montage|PlayMontage (Variables|Default|GetMesh) "/Game/Animations/Assets/Mixamo/Taunts/AM_LeftFighterIntro.AM_LeftFighterIntro"))

(event EventDie
  (Utilities|HandleDeath))

(fn ConstructionScript)

(fn IncreaseDamageAmp
  (params (amount :type Float%20%28double-precision%29)))

(fn InitialiseAttacks
  (Variables|/Game/Blueprints/AC_AttackManager.AC_AttackManager_C|SetstandingAttacks (Variables|Default|GetAttackManager) (Utilities|Array|MakeArray (Utilities|Struct|MakeAttack "/Game/Animations/Assets/Mixamo/Attacks/LeftPunch_Montage.LeftPunch_Montage" 2e+01 "LeftHand" true false "High" "/Game/Inputs/IA_L1.IA_L1" 1.0) (Utilities|Struct|MakeAttack "/Game/Animations/Assets/Mixamo/Attacks/Leg_Sweep_Montage.Leg_Sweep_Montage" 3e+01 "RightFoot" true false "Low" "/Game/Inputs/IA_R1.IA_R1" 2.0) (Utilities|Struct|MakeAttack "/Game/Animations/Assets/Mixamo/Attacks/RightKnee_Montage.RightKnee_Montage" 5e+01 "RightLeg" true false "High" "/Game/Inputs/IA_R2.IA_R2" 4.0))))

(fn GetHit
  (params (damage :type Float%20%28double-precision%29) (beatsToStun :type Float%20%28double-precision%29) (height :type AttackHeight%20Enum :default "None"))
  (bind _output_get (Variables|Stats|Sethealth (- (Variables|Stats|Gethealth) damage)))
  (if (<= _output_get 0.0)
    (Class|Fighter|Die)
    (else
      (Class|Fighter|Stun beatsToStun)
      (switch Utilities|FlowControl|Switch|SwitchonAttackHeight height ; Should be impossible to get None here
        (:Low
          (CallFunction|GetHitatHeight "NewEnumerator1"))
        (:High
          (if (Utilities|Enum|Equal(Enum) (Variables|/Script/Resonant.StateMachine|GetcurrentStateName (Variables|Default|GetstateMachine)) "Jumping") :!label _label ; If jumping and incoming high or aerial attack, get knocked out of air
            (CallFunction|GetHitatHeight "NewEnumerator0")
            (else
              (CallFunction|GetHitatHeight "NewEnumerator2"))))
        (:Aerial
          (goto _label))))))