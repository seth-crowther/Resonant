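; Player character Blueprint for a side-view fighter with beat-timed attacks, handling movement, health and attack input.
; Tick drives hand-written swept movement along Y: walking when grounded, gravity-driven jumps that keep their takeoff direction, landing on flat-surface hits.
; Punch and knee inputs go to AttackManager, whose on-beat state gates damage amplifier gains.
; At zero health, it plays a death montage, then restores health.
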(event Input|EnhancedActionEvents|EnhancedInputActionIA_LeftLight
  (params (ActionValue :type Boolean) (ElapsedSeconds :type Float%20%28double-precision%29) (TriggeredSeconds :type Float%20%28double-precision%29) (InputAction :type Input%20Action%20Object%20Reference :default "/Game/Inputs/IA_LeftLight.IA_LeftLight"))
  ;[1 1 1] Left Punch Attack
  (:Started
    (Default|AttackInput (Variables|Default|GetAttackManager) "NewEnumerator0")))

(event Input|EnhancedActionEvents|EnhancedInputActionIA_RightHeavy
  (params (ActionValue :type Boolean) (ElapsedSeconds :type Float%20%28double-precision%29) (TriggeredSeconds :type Float%20%28double-precision%29) (InputAction :type Input%20Action%20Object%20Reference :default "/Game/Inputs/IA_RightHeavy.IA_RightHeavy"))
  ;[1 1 1] Right Knee Attack
  (:Started
    (Default|AttackInput (Variables|Default|GetAttackManager) "NewEnumerator1")))

(event Input|EnhancedActionEvents|EnhancedInputActionIA_Move
  (params (ActionValue :type Float%20%28double-precision%29) (ElapsedSeconds :type Float%20%28double-precision%29) (TriggeredSeconds :type Float%20%28double-precision%29) (InputAction :type Input%20Action%20Object%20Reference :default "/Game/Inputs/IA_Move.IA_Move"))
  ;[1 1 1] Getting Left Stick Input
  (:Triggered
    (if (> ActionValue 0.0)
      (Variables|Input|SethorizontalInputDir 1)
      (else
        (Variables|Input|SethorizontalInputDir -1))))
  (:Completed
    (Variables|Input|SethorizontalInputDir 0)))

(event Input|EnhancedActionEvents|EnhancedInputActionIA_Jump
  (params (ActionValue :type Boolean) (ElapsedSeconds :type Float%20%28double-precision%29) (TriggeredSeconds :type Float%20%28double-precision%29) (InputAction :type Input%20Action%20Object%20Reference :default "/Game/Inputs/IA_Jump.IA_Jump"))
  ;[1 1 1] Handle Jumping
  (:Started
    (if (Variables|Movement|GetisGrounded)
      (Variables|Movement|SetzSpeed 4e+02)
      (Variables|Movement|SetisGrounded false)
      (Variables|Movement|SetlastHorizontalDir (Variables|Input|GethorizontalInputDir)))))

(event EventBeginPlay
  (Utilities|FlowControl|Sequence
    (:then_0
      (Variables|Stats|Sethealth (Variables|Stats|GetmaxHealth)))))

(event EventTick
  (params (DeltaSeconds :type Float%20%28single-precision%29))
  ;[1 1 1] Update
  (if (<= (Variables|Stats|Gethealth) 0.0)
    (Utilities|FlowControl|DoOnce false :!label _label
      (:Completed
        (Utilities|Die
          (:Completed
            (Variables|Stats|Sethealth 1e+02)
            (goto _label Reset)))))
    (elif (Variables|Movement|GetisGrounded)
      (if (not (Variables|Movement|GetimmobilizeHorizontal))
        (CallFunction|HandleGroundedMovement DeltaSeconds))
      (else
        (CallFunction|HandleAirborneMovement DeltaSeconds)))))

(event Collision|EventHit
  (params (MyComp :type Primitive%20Component%20Object%20Reference) (Other :type Actor%20Object%20Reference) (OtherComp :type Primitive%20Component%20Object%20Reference) (bSelfMoved :type Boolean) (HitLocation :type Vector :default "0, 0, 0") (HitNormal :type Vector :default "0, 0, 0") (NormalImpulse :type Vector :default "0, 0, 0") (Hit :type Hit%20Result%20Structure%20%28by%20ref%29))
  ;[1 1 1] Reset Z Speed When Hitting Ground
  (if (and (< (Variables|Movement|GetzSpeed) 0.0) (== (.Z (Class|KismetMathLibrary|BreakVector3f HitNormal)) 1.0))
    (Variables|Movement|SetzSpeed 0.0)
    (Variables|Movement|SetisGrounded true)))

(fn ConstructionScript)

(fn GetBrainBP
  (bind _outactors (Actor|GetAllActorsOfClass "/Game/Blueprints/Brain_BP.Brain_BP_C"))
  (Variables|Default|SetBrainBP (Utilities|Array|Get(acopy) _outactors)))

(fn HandleAirborneMovement
  (params (deltaTime :type Float%20%28double-precision%29))
  (bind _returnvalue (Transformation|GetActorLocation))
  (bind (_x _y _z) (Math|Vector|BreakVector _returnvalue))
  (Variables|Movement|SetzSpeed (+ (* (Variables|Constants|Getgravity) deltaTime) (Variables|Movement|GetzSpeed)))
  (Transformation|SetActorLocation (Math|Vector|MakeVector _x (+ _y (* deltaTime (Variables|Constants|GetwalkingSpeed) (Variables|Movement|GetlastHorizontalDir))) (+ _z (* (Variables|Movement|GetzSpeed) deltaTime))) true false))

(fn HandleGroundedMovement
  (params (deltaTime :type Float%20%28double-precision%29))
  (bind _returnvalue (Transformation|GetActorLocation))
  (bind (_x _y _z) (Math|Vector|BreakVector _returnvalue))
  (Transformation|SetActorLocation (Math|Vector|MakeVector _x (+ (* deltaTime (Variables|Constants|GetwalkingSpeed) (Variables|Input|GethorizontalInputDir)) _y) _z) true false))

(fn IncreaseDamageAmp
  (params (amount :type Float%20%28double-precision%29))
  (if (Variables|/Game/Blueprints/AttackManager.AttackManager_C|GetinputOnBeat (Variables|Default|GetAttackManager))
    (Variables|Stats|SetdamageAmplifier (Math|Float|Clamp(Float) (+ amount (Variables|Stats|GetdamageAmplifier)) 0.0 (Variables|Stats|GetmaxAmp)))))

(fn InitialiseMappingContext
  (bind _asplayer_controller (Utilities|Casting|CastToPlayerController (Pawn|GetController)))
  (Utilities|IsValid (PlayerController|LocalPlayerSubsystems|GetEnhancedInputLocalPlayerSubsystem _asplayer_controller)
    (:Is%20Valid
      (Input|AddMappingContext (PlayerController|LocalPlayerSubsystems|GetEnhancedInputLocalPlayerSubsystem _asplayer_controller) "/Game/Inputs/PlayerInputMappingContext.PlayerInputMappingContext" 0 "(bIgnoreAllPressedKeysUntilRelease=True,bForceImmediately=False)"))))