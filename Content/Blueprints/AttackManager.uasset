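; Attack manager for a character in a two-fighter rhythm fighting game, handling attack montages, hit detection and damage against the opponent.
; AttackInput maps an attack name to montage, damage, bone and horizontal lock, then plays it at a rate supplied by the Brain's Speaker.
; HitDetect sphere-traces at that bone once per hit flag, checking for blocks.
; On-beat hits raise the owner's damage amplifier; off-beat or premature inputs reset it.
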(event Custom|AttackInput
  (params (Attack :type Attacks%20Enum :default "NewEnumerator0"))
  (Utilities|ExecuteAttack Attack))

(event EventBeginPlay
  (CallFunction|GetBrainBP))

(fn ParseAttackName
  (params (AttackName :type Attacks%20Enum :default "NewEnumerator0"))
  (switch Utilities|FlowControl|Switch|SwitchonAttacks AttackName
    (:NewEnumerator0
      (return "/Game/Animations/Assets/Mixamo/Attacks/LeftPunch_Montage.LeftPunch_Montage" 2e+01 "LeftHand" true))
    (:NewEnumerator1
      (return "/Game/Animations/Assets/Mixamo/Attacks/RightKnee_Montage.RightKnee_Montage" 5e+01 "RightLeg" true))
    (:NewEnumerator2
      (return "/Game/Animations/Assets/Mixamo/Blocks/Mixamo_BlockIdle_Montage.Mixamo_BlockIdle_Montage" 0.0 "Head" false))))

(fn DamageOpponent
  (bind _opponent (Variables|Default|Getopponent))
  (bind _damage (CallFunction|ParseAttackName (Variables|Default|GetactiveAttack)))
  (Variables|/Game/Blueprints/Character_Blueprint.Character_Blueprint_C|Sethealth _opponent (- (Variables|/Game/Blueprints/Character_Blueprint.Character_Blueprint_C|Gethealth _opponent) (* _damage (+ (Variables|/Game/Blueprints/Character_Blueprint.Character_Blueprint_C|GetdamageAmplifier (Variables|Default|Getowner)) 1.0)))))

(fn GetBrainBP
  (bind _outactors (Actor|GetAllActorsOfClass "/Game/Blueprints/Brain_BP.Brain_BP_C"))
  (Variables|Default|SetBrain_BP (Utilities|Array|Get(acopy) _outactors)))

(fn InitialiseOwnerandOpponent
  (bind _brain_bp (Variables|Default|GetBrain_BP))
  (bind _leftcharacter (Variables|/Game/Blueprints/Brain_BP.Brain_BP_C|GetleftCharacter _brain_bp))
  (bind _rightcharacter (Variables|/Game/Blueprints/Brain_BP.Brain_BP_C|GetrightCharacter _brain_bp))
  (if (== (Components|GetOwner) _leftcharacter)
    (Variables|Default|Setowner _leftcharacter)
    (Variables|Default|Setopponent _rightcharacter)
    (else
      (Variables|Default|Setowner _rightcharacter)
      (Variables|Default|Setopponent _leftcharacter))))

(fn HitDetect
  (if (not (Variables|Default|GethasHitAlready))
    (bind _targetbone (CallFunction|ParseAttackName (Variables|Default|GetactiveAttack)))
    (bind _outhit (Collision|SphereTraceForObjects (Transformation|GetSocketLocation (Variables|/Game/Blueprints/Character_Blueprint.Character_Blueprint_C|GetMesh (Variables|Default|Getowner)) _targetbone) (Transformation|GetSocketLocation (Variables|/Game/Blueprints/Character_Blueprint.Character_Blueprint_C|GetMesh (Variables|Default|Getowner)) _targetbone) 1e+01 (Utilities|Array|MakeArray "ObjectTypeQuery3") false 0 "ForDuration"))
    (Utilities|IsValid (.HitComponent (Collision|BreakHitResult _outhit))
      (:Is%20Valid
        (if (== (Components|GetOwner (.HitComponent (Collision|BreakHitResult _outhit))) (Variables|Default|Getopponent))
          (if (Variables|AttackManager_C|GetisBlocking (Variables|/Game/Blueprints/Character_Blueprint.Character_Blueprint_C|GetAttackManager (Variables|Default|Getopponent)))
            _
            (else
              (Variables|Default|SethasHitAlready true)
              (if (Variables|Default|GetinputOnBeat)
                (Default|IncreaseDamageAmp (Variables|Default|Getowner) 0.1))
              (return true))))
        (Variables|Default|SethasHitAlready true)
        (Development|PrintString "Blocked")
        (return false))
      (:Is%20Not%20Valid
        (return false)))))

(fn ResetAmp
  (Variables|/Game/Blueprints/Character_Blueprint.Character_Blueprint_C|SetdamageAmplifier (Variables|Default|Getowner) 0.0)
  (Variables|Default|SetinputOnBeat false))