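; Speaker actor that plays audio and acts as the beat clock for rhythm-based gameplay.
; It derives playback time from the AudioComponent's playback-percent event, and each Tick sets OnBeat when that time falls within a threshold either side of a BPM interval.
; GetNewPlayRate returns a play rate that stretches or squeezes an attack animation to the nearest whole number of beats.
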(event Custom|OnAudioPlaybackPercent_Event
  (params (PlayingSoundWave :type Sound%20Wave%20Object%20Reference) (PlaybackPercent :type Float%20%28single-precision%29))
  (Variables|Default|SetplaybackTime (* (Variables|/Script/Engine.SoundBase|GetDuration PlayingSoundWave) PlaybackPercent)))

(event EventBeginPlay
  (bind _audiocomponent (Variables|Default|GetAudioComponent))
  (EventDispatchers|AssignOnAudioPlaybackPercent _audiocomponent (delegate Custom|OnAudioPlaybackPercent_Event))
  (Audio|Components|Audio|Play _audiocomponent 0.0))

(event EventTick
  (params (DeltaSeconds :type Float%20%28single-precision%29))
  (bind _onbeat (CallFunction|CheckBeat))
  (Variables|Default|SetonBeat _onbeat))

(fn ConstructionScript)

(fn CheckBeat
  (bind _playbacktime (Variables|Default|GetplaybackTime))
  (bind _onbeatthreshold (Variables|Default|GetonBeatThreshold))
  (bind _bpm (Variables|Default|Getbpm))
  (bind _returnvalue (/ 60 _bpm))
  (bind _remainder (Math|Float|Division(WholeandRemainder) _playbacktime _returnvalue))
  (return (or (< _remainder _onbeatthreshold) (> _remainder (- _returnvalue _onbeatthreshold)))))

(fn GetNewPlayRate
  (params (Attack :type Anim%20Montage%20Object%20Reference))
  (bind _bpm (Variables|Default|Getbpm))
  (bind _sequencelength (Variables|/Script/Engine.AnimSequenceBase|GetSequenceLength Attack))
  (bind _returnvalue (/ 6e+01 _bpm))
  (return (/ _sequencelength (* (Math|Float|Round (/ _sequencelength _returnvalue)) _returnvalue))))